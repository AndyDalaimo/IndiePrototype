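; BP_Eyes is an indicator actor that hovers above the player and turns its mesh to point toward the goal.
; On BeginPlay it caches the BP_Player and BP_Goal actors.
; Each tick it moves above the player and yaws the mesh by the acos of the flattened forward-to-goal dot product.
; A dot product with the right vector picks the side, mirroring the angle for a full 360-degree turn.
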(event EventBeginPlay
  (bind _returnvalue (Actor|GetActorOfClass "/Game/Blueprints/Player/BP_Player.BP_Player_C"))
  (Variables|Default|SetPlayerRef _returnvalue)
  (bind _returnvalue_2 (Actor|GetActorOfClass "/Game/Blueprints/BP_Goal.BP_Goal_C"))
  (Variables|Default|SetFinishRef _returnvalue_2))

(event EventTick
  (params (DeltaSeconds :type Float%20%28single-precision%29))
  (bind _returnvalue (Transformation|GetActorLocation))
  (bind _returnvalue_2 (Transformation|GetActorForwardVector))
  (bind _finishref (Variables|Default|GetFinishRef))
  (bind (_x _y) (Math|Vector|BreakVector _returnvalue))
  (bind (_x_2 _y_2) (Math|Vector|BreakVector _returnvalue_2))
  (bind _returnvalue_3 (Transformation|GetActorLocation _finishref))
  (bind (_x_3 _y_3) (Math|Vector|BreakVector _returnvalue_3))
  (bind _returnvalue_4 (Math|Vector|MakeVector _x _y 0.0))
  (bind _returnvalue_5 (Math|Vector|MakeVector _x_2 _y_2 0.0))
  (bind _returnvalue_6 (Math|Vector|MakeVector _x_3 _y_3 0.0))
  (bind _returnvalue_7 (Math|Vector|Normalize _returnvalue_5))
  (bind _returnvalue_8 (- _returnvalue_6 _returnvalue_4))
  (bind _returnvalue_9 (Math|Vector|Normalize _returnvalue_8))
  (bind _returnvalue_10 (Math|Vector|DotProduct _returnvalue_9 _returnvalue_7))
  (bind _returnvalue_11 (Math|Trig|Acos(Degrees) _returnvalue_10))
  (bind _returnvalue_12 (Math|Trig|RadiansToDegrees _returnvalue_11))
  (Transformation|SetActorLocation (+ (Transformation|GetActorLocation (Variables|Default|GetPlayerRef)) "0,0,150.000000") false false)
  (if (< (Math|Vector|DotProduct (Math|Vector|Normalize (- (Transformation|GetActorLocation (Variables|Default|GetFinishRef)) (Transformation|GetActorLocation))) (Math|Vector|Normalize (Transformation|GetActorRightVector))) 0.0)
    (Transformation|SetRelativeRotation (Variables|Default|GetStaticMesh) (Math|Rotator|MakeRotator 0.0 0.0 (- 3.6e+02 _returnvalue_12)) false false)
    (else
      (Transformation|SetRelativeRotation (Variables|Default|GetStaticMesh) (Math|Rotator|MakeRotator 0.0 0.0 _returnvalue_12) false false))))

(fn ConstructionScript)