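; BP_Spirit is a powerup pickup that restores a fixed amount of the player's Spirit.
; On BeginPlay it caches the BP_Player found in the level.
; When that player overlaps PickupCollider with enough headroom below an apparent 100-point cap, it adds Spirit, copies the value to the player's HUD and destroys itself.
; Otherwise the pickup stays in place.
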(event OnComponentBeginOverlap(PickupCollider)
  (params (OverlappedComponent :type Primitive%20Component%20Object%20Reference) (OtherActor :type Actor%20Object%20Reference) (OtherComp :type Primitive%20Component%20Object%20Reference) (OtherBodyIndex :type Integer) (bFromSweep :type Boolean) (SweepResult :type Hit%20Result%20Structure%20%28by%20ref%29))
  (bind _playerref (Variables|Default|GetPlayerRef))
  (if (and (== OtherActor (Variables|Default|GetPlayerRef)) (<= (Variables|/Game/Blueprints/Player/BP_Player.BP_Player_C|GetSpirit (Variables|Default|GetPlayerRef)) 9e+01))
    (bind _output_get (Variables|/Game/Blueprints/Player/BP_Player.BP_Player_C|SetSpirit _playerref (+ (Variables|/Game/Blueprints/Player/BP_Player.BP_Player_C|GetSpirit _playerref) 1e+01)))
    (Variables|/Game/Blueprints/UI/WBP_PlayerHUD.WBP_PlayerHUD_C|SetSpirit (Variables|/Game/Blueprints/Player/BP_Player.BP_Player_C|GetHUDRef _playerref) _output_get)
    (Actor|DestroyActor)))

(event EventBeginPlay
  (bind _returnvalue (Actor|GetActorOfClass "/Game/Blueprints/Player/BP_Player.BP_Player_C"))
  (Variables|Default|SetPlayerRef _returnvalue))

(fn ConstructionScript)