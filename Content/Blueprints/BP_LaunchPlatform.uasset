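; BP_LaunchPlatform is a launch pad that throws the player character upward on contact.
; It caches the BP_Player actor at BeginPlay and reacts only when that actor overlaps the Launchpad component.
; The overlap raises the player's GravityScale, never restoring it here, then calls LaunchCharacter with a multiple of JumpZVelocity, overriding vertical velocity.
; A debug print shows the base JumpZVelocity rather than the launch speed.
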(event OnComponentBeginOverlap(Launchpad)
  (params (OverlappedComponent :type Primitive%20Component%20Object%20Reference) (OtherActor :type Actor%20Object%20Reference) (OtherComp :type Primitive%20Component%20Object%20Reference) (OtherBodyIndex :type Integer) (bFromSweep :type Boolean) (SweepResult :type Hit%20Result%20Structure%20%28by%20ref%29))
  (bind _playerref (Variables|Default|GetPlayerRef))
  (bind _charactermovement (Variables|/Script/Engine.Character|GetCharacterMovement _playerref))
  (bind _jumpzvelocity (Variables|/Script/Engine.CharacterMovementComponent|GetJumpZVelocity _charactermovement))
  (if (== OtherActor (Variables|Default|GetPlayerRef))
    (Variables|/Script/Engine.CharacterMovementComponent|SetGravityScale _charactermovement 6.0)
    (Character|LaunchCharacter _playerref (Math|Vector|MakeVector 0.0 0.0 (* _jumpzvelocity 3.0)) false true)
    (Development|PrintString (Utilities|String|Append "Player z velocity: " (Utilities|String|ToString(Float) _jumpzvelocity)))))

(event EventBeginPlay
  (bind _returnvalue (Actor|GetActorOfClass "/Game/Blueprints/BP_Player.BP_Player_C"))
  (Variables|Default|SetPlayerRef _returnvalue))

(fn ConstructionScript)