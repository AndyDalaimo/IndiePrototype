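; BP_KeyItem is a key item pickup that starts an inspection camera view when the player overlaps its collider.
; The overlap flags the player as inspecting, passes the item's Index, stops movement and blends the view to the shared BP_KeyItemCam.
; The camera takes the player's KeyItemCamPos at the item's height.
; UpdateKeyItem, not called within this Blueprint, destroys the pickup's components and increments the player and HUD key item count.
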(event OnComponentBeginOverlap(PickupCollider)
  (params (OverlappedComponent :type Primitive%20Component%20Object%20Reference) (OtherActor :type Actor%20Object%20Reference) (OtherComp :type Primitive%20Component%20Object%20Reference) (OtherBodyIndex :type Integer) (bFromSweep :type Boolean) (SweepResult :type Hit%20Result%20Structure%20%28by%20ref%29))
  (if (== OtherActor (Variables|Default|GetPlayerRef))
    (Variables|/Game/Blueprints/Player/BP_Player.BP_Player_C|SetinspectingItem (Variables|Default|GetPlayerRef) true)
    (Default|SetChestIndex (Variables|Default|GetPlayerRef) (Variables|Default|GetIndex))
    (CallFunction|ActivateCamera)))

(event EventBeginPlay
  (bind _returnvalue (Actor|GetActorOfClass "/Game/Blueprints/Player/BP_Player.BP_Player_C"))
  (Variables|Default|SetPlayerRef _returnvalue)
  (bind _returnvalue_2 (Actor|GetActorOfClass "/Game/Blueprints/Cameras/BP_KeyItemCam.BP_KeyItemCam_C"))
  (Variables|Default|SetCameraRef _returnvalue_2))

(event Collision|EventActorBeginOverlap
  (params (OtherActor :type Actor%20Object%20Reference)))

(event EventTick
  (params (DeltaSeconds :type Float%20%28single-precision%29)))

(fn ConstructionScript)

(fn UpdateKeyItem
  (bind _playerref (Variables|Default|GetPlayerRef))
  (Components|DestroyComponent (Variables|Default|GetSphere))
  (Components|DestroyComponent (Variables|Default|GetPointLight))
  (Components|DestroyComponent (Variables|Default|GetPickupCollider))
  (bind _result (Math|Integer|IncrementInt (Variables|/Game/Blueprints/Player/BP_Player.BP_Player_C|GetKeyItems _playerref))
    (:%20%20
      (Variables|/Game/Blueprints/UI/WBP_PlayerHUD.WBP_PlayerHUD_C|SetKeyItems (Variables|/Game/Blueprints/Player/BP_Player.BP_Player_C|GetHUDRef _playerref) _result))))

(fn ActivateCamera
  (bind _playerref (Variables|Default|GetPlayerRef))
  (bind _keyitemcampos (Variables|/Game/Blueprints/Player/BP_Player.BP_Player_C|GetKeyItemCamPos _playerref))
  (bind _returnvalue (Transformation|GetWorldLocation _keyitemcampos))
  (Variables|/Game/Blueprints/Cameras/BP_KeyItemCam.BP_KeyItemCam_C|SetcamActive (Variables|Default|GetCameraRef) true)
  (Pawn|Components|CharacterMovement|SetMovementMode (Variables|/Script/Engine.Character|GetCharacterMovement (Variables|Default|GetPlayerRef)) "MOVE_None" 0)
  (Transformation|SetWorldLocationAndRotation (Variables|/Script/Engine.Actor|GetRootComponent (Variables|Default|GetCameraRef)) (Math|Vector|MakeVector (.x _returnvalue) (.y _returnvalue) (.z (Transformation|GetActorLocation))) (Transformation|GetWorldRotation _keyitemcampos) true false)
  (Game|Player|SetViewTargetwithBlend (Game|GetPlayerController 0) (Variables|Default|GetCameraRef) 1.8 "VTBlend_Linear" 0.5 false))