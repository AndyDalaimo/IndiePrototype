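; BP_SpiritWell is a pickup actor that restores the player's Spirit when they enter its InteractTrigger.
; It caches BP_Player on BeginPlay and compares overlapping actors against that reference.
; UpdateSpirit adds a fixed amount if Spirit is below its cap, clamps the result and writes it directly to the player's HUD reference.
; The well has no cooldown or depletion, and its fountain sound node is disconnected.
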(event OnComponentBeginOverlap(InteractTrigger)
  (params (OverlappedComponent :type Primitive%20Component%20Object%20Reference) (OtherActor :type Actor%20Object%20Reference) (OtherComp :type Primitive%20Component%20Object%20Reference) (OtherBodyIndex :type Integer) (bFromSweep :type Boolean) (SweepResult :type Hit%20Result%20Structure%20%28by%20ref%29))
  (if (== OtherActor (Variables|Default|GetPlayerRef))
    (CallFunction|UpdateSpirit)))

(event EventBeginPlay
  (bind _returnvalue (Actor|GetActorOfClass "/Game/Blueprints/Player/BP_Player.BP_Player_C"))
  (Variables|Default|SetPlayerRef _returnvalue))

(event Collision|EventActorBeginOverlap
  (params (OtherActor :type Actor%20Object%20Reference)))

(event EventTick
  (params (DeltaSeconds :type Float%20%28single-precision%29)))

(fn ConstructionScript)

(fn UpdateSpirit
  (bind _playerref (Variables|Default|GetPlayerRef))
  (bind _playerref_2 (Variables|Default|GetPlayerRef))
  (Development|PrintString "interact with spirit well")
  (if (< (Variables|/Game/Blueprints/Player/BP_Player.BP_Player_C|GetSpirit (Variables|Default|GetPlayerRef)) 1e+02)
    (bind _output_get (Variables|/Game/Blueprints/Player/BP_Player.BP_Player_C|SetSpirit _playerref_2 (+ (Variables|/Game/Blueprints/Player/BP_Player.BP_Player_C|GetSpirit (Variables|Default|GetPlayerRef)) 5e+01)))
    (if (> _output_get 1e+02)
      (bind _output_get_2 (Variables|/Game/Blueprints/Player/BP_Player.BP_Player_C|SetSpirit _playerref 1e+02))
      (Variables|/Game/Blueprints/UI/WBP_PlayerHUD.WBP_PlayerHUD_C|SetSpirit (Variables|/Game/Blueprints/Player/BP_Player.BP_Player_C|GetHUDRef _playerref) _output_get_2)
      (else
        (Variables|/Game/Blueprints/UI/WBP_PlayerHUD.WBP_PlayerHUD_C|SetSpirit (Variables|/Game/Blueprints/Player/BP_Player.BP_Player_C|GetHUDRef _playerref_2) _output_get)))))