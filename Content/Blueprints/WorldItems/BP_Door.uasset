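; BP_Door is a level-exit portal that lets the player leave once they carry at least three key items.
; BeginPlay caches the player and pre-creates the WBP_ExitLevel widget.
; Overlapping the PortalEntrance component checks the player's KeyItems count and calls ActivatePortal, which shows the exit widget, disables input and stops character movement.
; Debug strings report each outcome.
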(event OnComponentBeginOverlap(PortalEntrance)
  (params (OverlappedComponent :type Primitive%20Component%20Object%20Reference) (OtherActor :type Actor%20Object%20Reference) (OtherComp :type Primitive%20Component%20Object%20Reference) (OtherBodyIndex :type Integer) (bFromSweep :type Boolean) (SweepResult :type Hit%20Result%20Structure%20%28by%20ref%29))
  (if (== OtherActor (Variables|Default|GetPlayerRef))
    (Development|PrintString "Player in Portal")
    (if (>= (Variables|/Game/Blueprints/Player/BP_Player.BP_Player_C|GetKeyItems (Variables|Default|GetPlayerRef)) 3)
      (CallFunction|ActivatePortal)
      (else
        (Development|PrintString "Player CANNOT travel")))))

(event EventBeginPlay
  (bind _returnvalue (Actor|GetActorOfClass "/Game/Blueprints/Player/BP_Player.BP_Player_C"))
  (Variables|Default|SetPlayerRef _returnvalue)
  (bind _returnvalue_2 (UserInterface|CreateWidget "/Game/Blueprints/UI/WBP_ExitLevel.WBP_ExitLevel_C"))
  (Variables|Default|SetExitUIRef _returnvalue_2))

(event Collision|EventActorBeginOverlap
  (params (OtherActor :type Actor%20Object%20Reference)))

(event EventTick
  (params (DeltaSeconds :type Float%20%28single-precision%29)))

(fn ConstructionScript)

(fn ActivatePortal
  (bind _playerref (Variables|Default|GetPlayerRef))
  (Development|PrintString "Portal Active")
  (UserInterface|Viewport|AddtoViewport (Variables|Default|GetExitUIRef) 0)
  (Input|DisableInput _playerref (Game|GetPlayerController 0))
  (Pawn|Components|CharacterMovement|SetMovementMode (Variables|/Script/Engine.Character|GetCharacterMovement _playerref) "MOVE_None" 0))