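; BP_MantlePlatform is a platform that lets a climbing BP_Player mantle onto it through its MantleCollider.
; On overlap, a downward sphere trace ahead of the player's head finds the landing spot, with persistent debug drawing.
; It sets the player's Mantle flag, disables movement, then after a fixed delay snaps the player there and restores walking.
; A lerp-based move is left unconnected.
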(event OnComponentBeginOverlap(MantleCollider)
  (params (OverlappedComponent :type Primitive%20Component%20Object%20Reference) (OtherActor :type Actor%20Object%20Reference) (OtherComp :type Primitive%20Component%20Object%20Reference) (OtherBodyIndex :type Integer) (bFromSweep :type Boolean) (SweepResult :type Hit%20Result%20Structure%20%28by%20ref%29))
  (bind _playerref (Variables|Default|GetPlayerRef))
  (bind _playerref_2 (Variables|Default|GetPlayerRef))
  (if (and (== OtherActor _playerref_2) (Variables|/Game/Blueprints/Player/BP_Player.BP_Player_C|GetisClimbing _playerref_2))
    (CallFunction|DetermineClimbLoc)
    (Variables|/Game/Blueprints/Player/BP_Player.BP_Player_C|Setmantle _playerref true)
    (Pawn|Components|CharacterMovement|DisableMovement (Variables|/Script/Engine.Character|GetCharacterMovement _playerref))
    (Utilities|FlowControl|Delay 1.2)
    (Transformation|SetActorLocation (Variables|Default|GetPlayerRef) (Variables|Default|GetclimbLoc) false false)
    (Pawn|Components|CharacterMovement|SetMovementMode (Variables|/Script/Engine.Character|GetCharacterMovement (Variables|Default|GetPlayerRef)) "MOVE_Walking" 0)))

(event EventBeginPlay
  (bind _returnvalue (Actor|GetActorOfClass "/Game/Blueprints/Player/BP_Player.BP_Player_C"))
  (Variables|Default|SetPlayerRef _returnvalue))

(event Collision|EventActorBeginOverlap
  (params (OtherActor :type Actor%20Object%20Reference)))

(event EventTick
  (params (DeltaSeconds :type Float%20%28single-precision%29)))

(fn ConstructionScript)

(fn DetermineClimbLoc
  (bind _playerref (Variables|Default|GetPlayerRef))
  (bind _returnvalue (Transformation|GetActorRotation _playerref))
  (bind _mesh (Variables|/Script/Engine.Character|GetMesh _playerref))
  (bind _returnvalue_2 (Transformation|GetSocketLocation _mesh "HeadTop_End"))
  (bind _returnvalue_3 (Math|Vector|GetForwardVector _returnvalue))
  (bind _returnvalue_4 (* _returnvalue_3 1e+02))
  (bind _returnvalue_5 (+ _returnvalue_4 _returnvalue_2))
  (bind (_outhit _returnvalue_6) (Collision|SphereTraceByChannel (Math|Vector|MakeVector (.x _returnvalue_5) (.y _returnvalue_5) (+ (.z _returnvalue_5) 75.0)) (+ _returnvalue_4 _returnvalue_2) 5.0 "TraceTypeQuery1" false 0 "Persistent"))
  (if _returnvalue_6
    (Variables|Default|SetclimbLoc (+ (.ImpactPoint (Collision|BreakHitResult _outhit)) "0,0,50.000000"))))