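; BP_LaunchPlatform is a bounce pad that launches the player upward when they overlap its Launchpad component.
; The launch sets gravity scale high without restoring it here, overrides vertical velocity with boosted jump velocity, and plays a bounce sound and spirit effect.
; SetLaunchVelo stores optional horizontal velocity for the next launch, which resets to zero after use.
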(event OnComponentBeginOverlap(Launchpad)
  (params (OverlappedComponent :type Primitive%20Component%20Object%20Reference) (OtherActor :type Actor%20Object%20Reference) (OtherComp :type Primitive%20Component%20Object%20Reference) (OtherBodyIndex :type Integer) (bFromSweep :type Boolean) (SweepResult :type Hit%20Result%20Structure%20%28by%20ref%29))
  (bind _playerref (Variables|Default|GetPlayerRef))
  (bind _charactermovement (Variables|/Script/Engine.Character|GetCharacterMovement _playerref))
  (if (== OtherActor (Variables|Default|GetPlayerRef))
    (Variables|/Script/Engine.CharacterMovementComponent|SetGravityScale _charactermovement 6.0)
    (Character|LaunchCharacter (Variables|Default|GetPlayerRef) (Math|Vector|MakeVector (Variables|Default|GetXVelo) (Variables|Default|GetYVelo) (* (Variables|/Script/Engine.CharacterMovementComponent|GetJumpZVelocity _charactermovement) 2.5)) false true)
    (Audio|SpawnSoundatLocation "/Game/Sounds/bounce.bounce" (Transformation|GetActorLocation) "0, 0, 0" 1.0 1.0 0.0 0 0)
    (Variables|Default|SetYVelo 0.0)
    (Variables|Default|SetXVelo 0.0)
    (Niagara|SpawnSystematLocation "/Game/Blueprints/Pickups/P_SpiritFX.P_SpiritFX" (+ (Transformation|GetActorLocation) "0,0,120.000000"))))

(event EventBeginPlay
  (bind _returnvalue (Actor|GetActorOfClass "/Game/Blueprints/Player/BP_Player.BP_Player_C"))
  (Variables|Default|SetPlayerRef _returnvalue))

(fn ConstructionScript)

(fn SetLaunchVelo
  (params (X :type Float%20%28double-precision%29) (Y :type Float%20%28double-precision%29))
  (Variables|Default|SetXVelo X)
  (Variables|Default|SetYVelo Y))