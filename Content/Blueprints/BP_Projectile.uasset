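; Teleport projectile held in front of the player while aiming, gaining power over time until Shoot launches it along the camera direction.
; Each tick it predicts the arc, feeding a spline, trail effect and endpoint marker, and turns the player with the camera.
; Aiming at a launch platform also sets that platform's horizontal launch velocity.
; Any overlap re-enables shooting and destroys it; teleport platforms first send the player to the predicted point.
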(event OnComponentBeginOverlap(Sphere)
  (params (OverlappedComponent :type Primitive%20Component%20Object%20Reference) (OtherActor :type Actor%20Object%20Reference) (OtherComp :type Primitive%20Component%20Object%20Reference) (OtherBodyIndex :type Integer) (bFromSweep :type Boolean) (SweepResult :type Hit%20Result%20Structure%20%28by%20ref%29))
  (bind _playerref (Variables|Default|GetPlayerRef))
  (bind _playerref_2 (Variables|Default|GetPlayerRef))
  (if (Actor|ActorHasTag OtherActor "TP_Platform")
    (Default|TeleportPlayer (Variables|Default|GetPlayerRef) (Variables|Default|GetnewPlayerLoc) (Variables|Default|GetPoints))
    (Variables|/Game/Blueprints/Player/BP_Player.BP_Player_C|SetisFiring _playerref_2 false)
    (Variables|/Game/Blueprints/Player/BP_Player.BP_Player_C|SetCanShoot _playerref_2 true)
    (Actor|DestroyActor)
    (else
      (Variables|/Game/Blueprints/Player/BP_Player.BP_Player_C|SetisFiring _playerref false)
      (Variables|/Game/Blueprints/Player/BP_Player.BP_Player_C|SetCanShoot _playerref true)
      (Actor|DestroyActor))))

(event Custom|AddPower
  (Variables|Default|SetPower (+ (Math|Float|Clamp(Float) (Variables|Default|GetPower) 0.0 5.0) 0.05)))

(event EventBeginPlay
  (Rendering|SetVisibility (Variables|Default|GetSphere) false false)
  (bind _returnvalue (Actor|GetActorOfClass "/Game/Blueprints/Player/BP_Player.BP_Player_C"))
  (bind _output_get (Variables|Default|SetPlayerRef _returnvalue))
  (Variables|/Game/Blueprints/Player/BP_Player.BP_Player_C|SetCanShoot _output_get false)
  (bind _outactors (Actor|GetAllActorsOfClass "/Game/Blueprints/BP_Platform.BP_Platform_C"))
  (Variables|Default|SetPlatformRef _outactors)
  (bind _returnvalue_2 (Actor|GetActorOfClass "/Game/Blueprints/BP_LaunchPlatform.BP_LaunchPlatform_C"))
  (Variables|Default|SetLaunchPlatRef _returnvalue_2)
  (Utilities|Time|SetTimerbyEvent (delegate Custom|AddPower) 0.01 true))

(event EventTick
  (params (DeltaSeconds :type Float%20%28single-precision%29))
  (bind _playerref (Variables|Default|GetPlayerRef))
  (bind _playerref_2 (Variables|Default|GetPlayerRef))
  (bind _points (Variables|Default|GetPoints))
  (bind _followcamera (Variables|/Game/Blueprints/Player/BP_Player.BP_Player_C|GetFollowCamera _playerref_2))
  (bind _returnvalue (Transformation|GetSocketRotation _followcamera "None"))
  (Transformation|SetWorldRotation (Variables|/Script/Engine.Character|GetCapsuleComponent _playerref_2) (Math|Rotator|MakeRotator (.roll _returnvalue) 0.0 (.yaw _returnvalue)) false false)
  (if (Variables|/Game/Blueprints/Player/BP_Player.BP_Player_C|GetisFiring _playerref)
    (Transformation|SetActorLocation (+ (Transformation|GetActorLocation _playerref) (* (Math|Vector|GetForwardVector (Transformation|GetSocketRotation (Variables|/Game/Blueprints/Player/BP_Player.BP_Player_C|GetThrowingPosition _playerref) "None")) 2e+02)) false false))
  (bind (_outhit _outpathpositions) (Class|GameplayStatics|BlueprintPredictProjectilePathbyTraceChannel (Transformation|GetActorLocation) (* (* (Math|Vector|GetForwardVector (Variables|/Game/Blueprints/Player/BP_Player.BP_Player_C|GetFollowCamera (Variables|Default|GetPlayerRef))) (Variables|/Script/Engine.ProjectileMovementComponent|GetInitialSpeed (Variables|Default|GetProjectileMovement))) (Variables|Default|GetPower)) true 5.0 "ECC_WorldDynamic" false 0 "None"))
  (Spline|SetSplinePoints _points _outpathpositions "Local" true)
  (Effects|Components|ParticleSystem|SetVectorParameter (Variables|Default|GetSplineFX) "Start" (Spline|GetLocationatSplinePoint _points 0 "Local"))
  (Effects|Components|ParticleSystem|SetVectorParameter (Variables|Default|GetSplineFX) "Start_Tangent" (Spline|GetLocationatSplinePoint (Variables|Default|GetPoints) 2 "Local"))
  (Effects|Components|ParticleSystem|SetVectorParameter (Variables|Default|GetSplineFX) "End_Tangent" (Spline|GetLocationatSplinePoint (Variables|Default|GetPoints) 6 "Local"))
  (Effects|Components|ParticleSystem|SetVectorParameter (Variables|Default|GetSplineFX) "End" (Spline|GetLocationatSplinePoint (Variables|Default|GetPoints) 8 "Local"))
  (if (.bBlockingHit (Collision|BreakHitResult _outhit))
    (if (Actor|ActorHasTag (.HitActor (Collision|BreakHitResult _outhit)) "Launch_Platform")
      (bind (_x _y) (CallFunction|DetermineLaunchVelocity (Transformation|GetActorLocation (Variables|Default|GetPlayerRef)) (Transformation|GetActorLocation (.HitActor (Collision|BreakHitResult _outhit)))))
      (Default|SetLaunchVelo (Variables|Default|GetLaunchPlatRef) _x _y)
      (Variables|Default|SetnewPlayerLoc (Math|Vector|MakeVector (.x (.ImpactPoint (Collision|BreakHitResult _outhit))) (.y (.ImpactPoint (Collision|BreakHitResult _outhit))) (+ (.z (.ImpactPoint (Collision|BreakHitResult _outhit))) 5e+01)))
      (else
        (bind _output_get (Variables|Default|SetnewPlayerLoc (Math|Vector|MakeVector (.x (.ImpactPoint (Collision|BreakHitResult _outhit))) (.y (.ImpactPoint (Collision|BreakHitResult _outhit))) (.z (.ImpactPoint (Collision|BreakHitResult _outhit))))))))
    (Transformation|SetWorldLocation (Variables|Default|GetEndpoint) _output_get false false)
    (Development|SetHiddeninGame (Variables|Default|GetEndpoint) false false)
    (else
      (Development|SetHiddeninGame (Variables|Default|GetEndpoint) true false))))

(fn ConstructionScript)

(fn Shoot
  (Rendering|SetVisibility (Variables|Default|GetSphere) true false)
  (Variables|/Script/Engine.MovementComponent|SetVelocity (Variables|Default|GetProjectileMovement) (* (* (Math|Vector|GetForwardVector (Variables|/Game/Blueprints/Player/BP_Player.BP_Player_C|GetFollowCamera (Variables|Default|GetPlayerRef))) (Variables|/Script/Engine.ProjectileMovementComponent|GetInitialSpeed (Variables|Default|GetProjectileMovement))) (Variables|Default|GetPower)))
  (Components|Activation|Activate (Variables|Default|GetProjectileMovement) false)
  (Variables|Default|SetFired true)
  (Development|SetHiddeninGame (Variables|Default|GetSplineFX) true false)
  (Development|SetHiddeninGame (Variables|Default|GetEndpoint) true false)
  (return))

(fn DetermineLaunchVelocity
  (params (Player :type Vector) (Platform :type Vector))
  (Variables|Default|SettempP Player)
  (Variables|Default|SettempL Platform)
  (if (< (.x (Variables|Default|GettempP)) (.x (Variables|Default|GettempL)))
    (Variables|Default|SettempV (Math|Vector|MakeVector (Math|Float|Absolute(Float) (- (.x (Variables|Default|GettempL)) (.x (Variables|Default|GettempP)))) 0.0 0.0))
    (else
      (Variables|Default|SettempV (Math|Vector|MakeVector (- (.x (Variables|Default|GettempL)) (.x (Variables|Default|GettempP))) 0.0 0.0))))
  (if (> (.y (Variables|Default|GettempP)) (.y (Variables|Default|GettempL)))
    (Variables|Default|SettempV (Math|Vector|MakeVector (.x (Variables|Default|GettempV)) (- (.y (Variables|Default|GettempL)) (.y (Variables|Default|GettempP))) 0.0))
    (else
      (Variables|Default|SettempV (Math|Vector|MakeVector (.x (Variables|Default|GettempV)) (Math|Float|Absolute(Float) (- (.y (Variables|Default|GettempL)) (.y (Variables|Default|GettempP)))) 0.0))))
  (return (.x (Variables|Default|GettempV)) (.y (Variables|Default|GettempV))))